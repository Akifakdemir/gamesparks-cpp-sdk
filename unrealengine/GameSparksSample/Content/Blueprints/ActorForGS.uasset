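; Test actor for GameSparks that puts a GameSparksTestMenu widget on screen at BeginPlay and keeps a reference to it.
; Its GameSparks component's log and availability events are bound but empty.
; An older BasicMenu logging path, which used AddLogMessage to append messages and availability status to a text box, remains disconnected and never runs.
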(event OnGameSparksAvailableDelegate(GameSparks1)
  (params (available :type Boolean)))

(event OnGameSparksLogEventDelegate(GameSparks1)
  (params (logMessage :type String))
  ;[1 1 1] When a wild debug log from gamesparks apears
)

(event EventBeginPlay
  (bind _returnvalue (UserInterface|CreateWidget "/Game/Menu/GameSparksTestMenu.GameSparksTestMenu_C"))
  (Variables|Default|SetMenuForTesting _returnvalue)
  (UserInterface|Viewport|AddtoViewport _returnvalue))

(fn ConstructionScript)

(fn AddLogMessage
  (params (message :type String) (textbox :type Multi%20Line%20Editable%20Text%20Box%20Object%20Reference))
  (Rendering|Components|TextRender|SetText textbox (Utilities|Text|ToText(String) (Utilities|String|Append (Utilities|String|ToString(Text) (Class|MultiLineEditableTextBox|GetText textbox)) message))))